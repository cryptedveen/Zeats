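; Interactable clock that starts the player's shift, triggering the SurvivalSpawner.
; Overlapping ShiftBox with a Hero-tagged GameBPI actor shows a prompt widget and enables input, so E or Interact can start it once.
; Starting sets a one-shot flag, begins a self-calling one-second delay loop that rotates the Larm hand, then calls SpawnStart after a short delay.
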(event OnComponentBeginOverlap(ShiftBox)
  (params (OverlappedComponent :type Primitive%20Component%20Object%20Reference) (OtherActor :type Actor%20Object%20Reference) (OtherComp :type Primitive%20Component%20Object%20Reference) (OtherBodyIndex :type Integer) (bFromSweep :type Boolean) (SweepResult :type Hit%20Result%20Structure%20%28by%20ref%29))
  (if (and (Actor|ActorHasTag OtherActor "Hero") (Utilities|DoesObjectImplementInterface OtherActor "/Game/GameBPs/BP_Interfaces/GameBPI.GameBPI_C"))
    (if (not (Variables|Default|GetSpawnStarted))
      (bind _returnvalue (UserInterface|CreateWidget "/Game/GameBPs/UIofGame/NotificationWidget.NotificationWidget_C"))
      (Rendering|Components|TextRender|SetText (Variables|/Game/GameBPs/UIofGame/NotificationWidget.NotificationWidget_C|GetNotify _returnvalue) "Enter E To Start Shift")
      (UserInterface|Viewport|AddtoViewport _returnvalue 0)
      (Input|EnableInput (Game|GetPlayerController 0)))))

(event OnComponentEndOverlap(ShiftBox)
  (params (OverlappedComponent :type Primitive%20Component%20Object%20Reference) (OtherActor :type Actor%20Object%20Reference) (OtherComp :type Primitive%20Component%20Object%20Reference) (OtherBodyIndex :type Integer))
  (if (and (Actor|ActorHasTag OtherActor "Hero") (Utilities|DoesObjectImplementInterface OtherActor "/Game/GameBPs/BP_Interfaces/GameBPI.GameBPI_C"))
    (Widget|RemovefromParent (stale OnComponentBeginOverlap(ShiftBox) _returnvalue))
    (Input|DisableInput (Game|GetPlayerController 0))))

(event Custom|ClockRun
  (bind _larm (Variables|Default|GetLarm))
  (Transformation|AddLocalRotation _larm (Math|Rotator|MakeRotator 0.0 0.0 (Math|Vector|VectorLength (+ (.Z (Math|Rotator|BreakRotIntoAxes (Transformation|GetWorldRotation _larm))) 2))) true false)
  (Utilities|FlowControl|Delay 1.0)
  (CallFunction|ClockRun))

(event EventInteract
  (params (Player :type ZE%20Hero%20Character%20Object%20Reference))
  (if (not (Variables|Default|GetSpawnStarted))
    (Variables|Default|SetSpawnStarted true)
    (CallFunction|ClockRun)
    (Utilities|FlowControl|Delay 2.0)
    (bind _returnvalue (Actor|GetActorOfClass "/Game/Zombies/SurvivalSpawner.SurvivalSpawner_C"))
    (Utilities|IsValid _returnvalue
      (:Is%20Valid
        (Default|SpawnStart _returnvalue)))))

(event Input|KeyboardEvents|E
  (params (Key :type Key%20Structure))
  (:Pressed
    (if (not (Variables|Default|GetSpawnStarted))
      (Variables|Default|SetSpawnStarted true)
      (CallFunction|ClockRun)
      (Utilities|FlowControl|Delay 2.0)
      (bind _returnvalue (Actor|GetActorOfClass "/Game/Zombies/SurvivalSpawner.SurvivalSpawner_C"))
      (Utilities|IsValid _returnvalue
        (:Is%20Valid
          (Default|SpawnStart _returnvalue))))))

(fn ConstructionScript)

(fn PickupItem
  (params (Player :type ZE%20Hero%20Character%20Object%20Reference))
  (return 0 0))